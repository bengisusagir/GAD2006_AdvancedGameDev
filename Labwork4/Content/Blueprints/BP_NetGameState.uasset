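; Game state Blueprint for a networked team game that handles the end-of-match result and restart.
; On victory, it compares each player's team to the WinningPlayer's, calling OnPlayerLost on same-team avatars and OnPlayerWon on others, seemingly inverted.
; It then shows W_GameResult, with blank winner text if the local player shares that team, otherwise naming the team.
; Restart removes the widget.
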(event EventOnVictory
  (bind _returnvalue (Class|NetGameState|GetPlayerStatebyIndex (Variables|Default|GetWinningPlayer)))
  (for _array_element (Variables|Default|GetPlayerArray)
    (bind _asnet_player_state (Utilities|Casting|CastToNetPlayerState _array_element))
    (if (Utilities|Enum|Equal(Enum) (.teamid (Variables|/Script/Labwork4.NetPlayerState|GetData _asnet_player_state)) (.TeamID (Utilities|Struct|BreakSPlayerInfo (Variables|/Script/Labwork4.NetPlayerState|GetData _returnvalue))))
      (Default|OnPlayerLost (.AsBP%20Net%20Avatar (Utilities|Casting|CastToBP_NetAvatar (Variables|/Script/Engine.PlayerState|GetPawnPrivate _asnet_player_state))))
      (else
        (Default|OnPlayerWon (.AsBP%20Net%20Avatar (Utilities|Casting|CastToBP_NetAvatar (Variables|/Script/Engine.PlayerState|GetPawnPrivate _asnet_player_state)))))))
  (CallFunction|ShowResultMessage))

(event EventOnRestart
  (Widget|RemovefromParent (Variables|Default|GetMessageWidget)))

(fn ConstructionScript)

(fn ShowResultMessage
  (bind _returnvalue (Class|NetGameState|GetPlayerStatebyIndex (Variables|Default|GetWinningPlayer)))
  (bind _returnvalue_2 (UserInterface|CreateWidget "/Game/Blueprints/UMG/W_GameResult.W_GameResult_C" 0 (select (Utilities|Enum|Equal(Enum) (.teamid (Variables|/Script/Labwork4.NetPlayerState|GetData _returnvalue)) (.teamid (Variables|/Script/Labwork4.NetPlayerState|GetData (.AsNet%20Player%20State (Utilities|Casting|CastToNetPlayerState (Variables|/Script/Engine.Controller|GetPlayerState (Game|GetPlayerController 0))))))) "" (Utilities|Text|FormatText "{team} WINS!" (Utilities|String|EnumtoString (.teamid (Variables|/Script/Labwork4.NetPlayerState|GetData _returnvalue)))))))
  (Variables|Default|SetMessageWidget _returnvalue_2)
  (UserInterface|Viewport|AddtoViewport _returnvalue_2 0))